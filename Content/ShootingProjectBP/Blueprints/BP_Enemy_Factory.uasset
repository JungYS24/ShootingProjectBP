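; BP_Enemy_Factory is a spawner actor that produces BP_Enemy instances at random intervals in the shooting project.
; BeginPlay picks a random delay between a fixed minimum and the MaxDelayTime variable.
; Tick accumulates elapsed time and, when it reaches the delay, spawns an enemy at the Spawnpoint component's world transform, resets the timer and rolls a new delay.
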(event EventTick
  (params (DeltaSeconds :type Float%20%28single-precision%29))
  (bind _output_get (Variables|Default|SetCurrentTime (+ DeltaSeconds (Variables|Default|GetCurrentTime))))
  (if (>= _output_get (Variables|Default|GetDelayTime))
    (Game|SpawnActorfromClass "/Game/ShootingProjectBP/Blueprints/BP_Enemy.BP_Enemy_C" (Transformation|GetWorldTransform (Variables|Default|Getspawnpoint)) "Undefined" "MultiplyWithRoot" 0 0)
    (Variables|Default|SetCurrentTime 0.0)
    (Variables|Default|SetDelayTime (Math|Random|RandomFloatinRange 0.3 (Variables|Default|GetMaxDelayTime)))))

(event EventBeginPlay
  (Variables|Default|SetDelayTime (Math|Random|RandomFloatinRange 0.3 (Variables|Default|GetMaxDelayTime))))

(fn ConstructionScript)