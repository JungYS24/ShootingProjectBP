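; Game mode for a shooting game that tracks the current score and a persistent best score.
; On BeginPlay it shows the WBP_Main widget and loads the saved best score.
; AddScore raises the current score and, when it beats the best, updates the best and immediately writes it to the BestScoreData slot through a BP_SaveScore save game object.
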(event EventBeginPlay
  (bind _returnvalue (UserInterface|CreateWidget "/Game/ShootingProjectBP/UI/WBP_Main.WBP_Main_C"))
  (UserInterface|Viewport|AddtoViewport _returnvalue 0)
  (bind _bestscore (CallFunction|LoadScoreData))
  (Variables|Default|SetBest_Score _bestscore))

(fn ConstructionScript)

(fn AddScore
  (params (Point :type Integer))
  (bind _output_get (Variables|Default|SetCurrentScore (+ Point (Variables|Default|GetCurrentScore))))
  (if (> _output_get (Variables|Default|GetBest_Score))
    (bind _output_get_2 (Variables|Default|SetBest_Score _output_get))
    (CallFunction|SaveScoreData _output_get_2)))

(fn SaveScoreData
  (params (Save%20Value :type Integer))
  (bind _returnvalue (SaveGame|CreateSaveGameObject "/Game/ShootingProjectBP/Blueprints/BP_SaveScore.BP_SaveScore_C"))
  (bind _output_get (Variables|Default|SetSaveInstance _returnvalue))
  (Variables|/Game/ShootingProjectBP/Blueprints/BP_SaveScore.BP_SaveScore_C|SetSaveScore _output_get Save%20Value)
  (SaveGame|SaveGametoSlot (Variables|Default|GetSaveInstance) "BestScoreData"))

(fn LoadScoreData
  (bind _returnvalue (SaveGame|DoesSaveGameExist "BestScoreData"))
  (if _returnvalue
    (bind _returnvalue_2 (SaveGame|LoadGamefromSlot "BestScoreData"))
    (bind _asbp_save_score (Utilities|Casting|CastToBP_SaveScore _returnvalue_2))
    (return (Variables|/Game/ShootingProjectBP/Blueprints/BP_SaveScore.BP_SaveScore_C|GetSaveScore _asbp_save_score))))