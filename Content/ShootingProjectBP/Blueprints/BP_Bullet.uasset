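; BP_Bullet is a projectile actor for a shooting game that destroys enemies and awards score.
; Each Tick it moves along its forward vector by MoveSpeed scaled by delta time, without sweeping.
; On overlap with a BP_Enemy it destroys the enemy, spawns an explosion emitter at its own location, adds a point through BP_Gamemodebase, then destroys itself.
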(event EventTick
  (params (DeltaSeconds :type Float%20%28single-precision%29))
  (Transformation|SetActorLocation (+ (Transformation|GetActorLocation) (* (* (Transformation|GetActorForwardVector) (Variables|Default|GetMoveSpeed)) DeltaSeconds)) false false))

(event Collision|EventActorBeginOverlap
  (params (OtherActor :type Actor%20Object%20Reference))
  ;[1 1 1] 들어온 actor클래스를 BP_ENEMY로 형변화
  (bind _asbp_enemy (Utilities|Casting|CastToBP_Enemy OtherActor))
  (Actor|DestroyActor _asbp_enemy)
  (Effects|SpawnEmitteratLocation "/Game/StarterContent/Particles/P_Explosion.P_Explosion" (Transformation|GetActorLocation))
  (bind _asbp_gamemodebase (Utilities|Casting|CastToBP_Gamemodebase (Game|GetGameMode)))
  (Default|AddScore _asbp_gamemodebase 1)
  (Actor|DestroyActor))

(fn ConstructionScript)