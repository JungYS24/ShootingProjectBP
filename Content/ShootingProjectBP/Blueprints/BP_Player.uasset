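; BP_Player is the player actor for a shooting project, moved by Enhanced Input on the world Y-Z plane.
; BeginPlay adds the IMC_PlayerInput mapping context to player 0.
; The IA_Horizontal and IA_Vertical actions store their values on both Triggered and Completed.
; Tick adds those values to the actor's location without sweep, speed scaling or delta time, so movement is frame-rate dependent.
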(event Input|EnhancedActionEvents|EnhancedInputActionIA_Horizontal
  (params (ActionValue :type Float%20%28double-precision%29) (ElapsedSeconds :type Float%20%28double-precision%29) (TriggeredSeconds :type Float%20%28double-precision%29) (InputAction :type Input%20Action%20Object%20Reference :default "/Game/ShootingProjectBP/Inputs/IA_Horizontal.IA_Horizontal"))
  ;[1 1 1] 수평 수직 이동
  (:Triggered
    (Variables|Default|SetHorizontal ActionValue))
  (:Completed
    (Variables|Default|SetHorizontal ActionValue)))

(event Input|EnhancedActionEvents|EnhancedInputActionIA_Vertical
  (params (ActionValue :type Float%20%28double-precision%29) (ElapsedSeconds :type Float%20%28double-precision%29) (TriggeredSeconds :type Float%20%28double-precision%29) (InputAction :type Input%20Action%20Object%20Reference :default "/Game/ShootingProjectBP/Inputs/IA_Vertical.IA_Vertical"))
  ;[1 1 1] 수평 수직 이동
  (:Triggered
    (Variables|Default|SetVertical ActionValue))
  (:Completed
    (Variables|Default|SetVertical ActionValue)))

(event EventBeginPlay
  ;[1 1 1] 수평 수직 이동
  (Input|AddMappingContext (PlayerController|LocalPlayerSubsystems|GetEnhancedInputLocalPlayerSubsystem (Game|GetPlayerController 0)) "/Game/ShootingProjectBP/Inputs/IMC_PlayerInput.IMC_PlayerInput" 0 "(bIgnoreAllPressedKeysUntilRelease=True,bForceImmediately=False,bNotifyUserSettings=False)"))

(event Collision|EventActorBeginOverlap
  (params (OtherActor :type Actor%20Object%20Reference)))

(event EventTick
  (params (DeltaSeconds :type Float%20%28single-precision%29))
  ;[1 1 1] 새위치로 이동
  (Transformation|SetActorLocation (+ (Transformation|GetActorLocation) (Math|Vector|MakeVector 0.0 (Variables|Default|GetHorizontal) (Variables|Default|GetVertical))) false false))

(fn ConstructionScript)